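; BP_Chest_02 is a reward chest that plays its open animation and spawns three 3D reward actors.
; After short delays, OpenChest spawns a gold reward, a shard reward using loot material from the character data table, and a third reward with default settings.
; It passes the spawned actors to the game mode's reward widget, cached at BeginPlay.
; Sphere overlap events are empty, and the close animation logic is unconnected.
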(event `self.ReceiveBeginPlay`
  (bind _asgotgame_mode (cast `/Game/Core/Blueprints/GOTGameMode` (`GameplayStatics.GetGameMode`)))
  (bind _output_get (set `self.Game ModeRef` _asgotgame_mode))
  (set `self.RewardWidget` (`/Game/Core/Blueprints/GOTGameMode.RewardWidgtRef` _output_get)))

(event `OpenChest`
  (bind _rewardwidget (`self.RewardWidget`))
  (`KismetSystemLibrary.Delay` 0.5)
  (`SkeletalMeshComponent.PlayAnimation` (`self.Chest`) "/Game/ChestFantasy/Meshes/Chest_02/Anim_Chest_02_Open.Anim_Chest_02_Open" false)
  (`KismetSystemLibrary.Delay` 1.0)
  (bind _returnvalue (`|SpawnActorFromClass` "/Game/3dReward.3dReward_C" (`KismetMathLibrary.MakeTransform` (`self.Reward1`) (struct :`Roll` -20.0) (0.25 0.25 0.25)) "Undefined" "OverrideRootScale" null "/Game/Core/UI/UI_Images/GoldMat_NonTrans.GoldMat_NonTrans" (`self.GoldAmount`) null))
  (bind _returnvalue_2 (`|GetDataTableRow` "/Game/Core/DataBPs/DataTable_CharacterTable.DataTable_CharacterTable" (`self.Name`))
    (:`then`
      (bind _returnvalue_3 (`|SpawnActorFromClass` "/Game/3dReward.3dReward_C" (`KismetMathLibrary.MakeTransform` (`self.Reward2`) (struct :`Roll` -20.0) (0.35 0.35 0.35)) "AlwaysSpawn" "OverrideRootScale" null (`.LootMat_62_C5ACE98D41BD77B9ED0AB99A7FB6DA81` (break `/Game/Core/DataBPs/Struct_CharInfo` _returnvalue_2)) (`self.ShardAmount`) null))
      (bind _returnvalue_4 (`|SpawnActorFromClass` "/Game/3dReward.3dReward_C" (`KismetMathLibrary.MakeTransform` (`self.Reward3`) (struct :`Roll` -20.0) (0.25 0.25 0.25)) "AlwaysSpawn" "OverrideRootScale" null null "" null)))
    (:`RowNotFound`
      _))
  (set `/Game/Core/UI/ShopUI/LootChestRewardsAnimated.RewardActor3` _returnvalue_4 _rewardwidget)
  (set `/Game/Core/UI/ShopUI/LootChestRewardsAnimated.RewardActor1` _returnvalue _rewardwidget)
  (set `/Game/Core/UI/ShopUI/LootChestRewardsAnimated.RewardActor2` _returnvalue_3 _rewardwidget))

(event `self.Sphere.OnComponentBeginOverlap`
  (params (OverlappedComponent :type "PrimitiveComponent Object Reference") (OtherActor :type "Actor Object Reference") (OtherComp :type "PrimitiveComponent Object Reference") (OtherBodyIndex :type Integer) (bFromSweep :type Boolean) (SweepResult :type "HitResult Structure (by ref)"))
  ;[1 1 1] Play animation
)

(event `self.Sphere.OnComponentEndOverlap`
  (params (OverlappedComponent :type "PrimitiveComponent Object Reference") (OtherActor :type "Actor Object Reference") (OtherComp :type "PrimitiveComponent Object Reference") (OtherBodyIndex :type Integer))
  ;[1 1 1] Play animation
)

(fn `UserConstructionScript`)