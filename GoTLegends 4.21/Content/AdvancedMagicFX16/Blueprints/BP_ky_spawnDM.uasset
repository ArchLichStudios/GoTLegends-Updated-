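; Spawnable destructible rock effect from the AdvancedMagicFX16 pack that shatters on spawn, fades out and removes itself.
; On BeginPlay it damages its own destructible component to trigger the break and creates dynamic materials for both material slots.
; After a short delay, a timeline drives their alpha parameter.
; A Delay fired from the timeline's update destroys the actor one second after the fade begins.
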(event `self.ReceiveBeginPlay`
  ;[1 1 1] damage to this OBJ
  ; because this destruction
  (`DestructibleComponent.ApplyDamage` (`self.DM_ky_rock`) 1.0 (`SceneComponent.K2_GetComponentLocation` (`self.DefaultSceneRoot`)) (+ (0.0 0.0 1.0) 0) 1.0)
  ;[1 1 1] get material inctance
  ; because it make fadeout
  (bind _returnvalue (`PrimitiveComponent.CreateDynamicMaterialInstance` (`self.DM_ky_rock`) 0 null))
  (bind _returnvalue_2 (`PrimitiveComponent.CreateDynamicMaterialInstance` (`self.DM_ky_rock`) 1 null))
  ;[1 1 1] one second after fadeout
  (`KismetSystemLibrary.Delay` 1.0)
  (bind (_direction _opacity) (`Timeline|Timeline_0` :!via `PlayFromStart`)
    (:`Update`
      (`MaterialInstanceDynamic.SetScalarParameterValue` _returnvalue "alphaValue" _opacity)
      (`MaterialInstanceDynamic.SetScalarParameterValue` _returnvalue_2 "alphaValue" _opacity)
      ;[1 1 1] this destroy
      (`KismetSystemLibrary.Delay` 1.0)
      (`self.K2_DestroyActor`))))

(event `self.ReceiveTick`
  (params (DeltaSeconds :type "Float (single-precision)")))

(fn `UserConstructionScript`)