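; Magic circle effect actor from the AdvancedMagicFX16 set, with editable colors for its main, inner circle, sub circle and line parts.
; The Construction Script pushes main, sub circle and line colors into the Fx component as vector parameters.
; The inner circle color instead goes through a dynamic material instance on Fx element 0.
; It has no active runtime logic, as the event graph holds only disabled placeholder events.
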(fn `UserConstructionScript`
  ;[1 1 1] main color control
  (`ParticleSystemComponent.SetVectorParameter` (`self.fx`) "color" (`KismetMathLibrary.Conv_LinearColorToVector` (`self.color`)))
  ;[1 1 1] in circle color control
  (bind _returnvalue (`PrimitiveComponent.CreateDynamicMaterialInstance` (`self.fx`) 0 null))
  (`MaterialInstanceDynamic.SetVectorParameterValue` _returnvalue "inColor" (`self.inCircleColor`))
  ;[1 1 1] sub circle color control
  (`ParticleSystemComponent.SetVectorParameter` (`self.fx`) "colorSub" (`KismetMathLibrary.Conv_LinearColorToVector` (`self.subCircleColor`)))
  ;[1 1 1] line color  control
  (`ParticleSystemComponent.SetVectorParameter` (`self.fx`) "colorLine" (`KismetMathLibrary.Conv_LinearColorToVector` (`self.lineColor`))))