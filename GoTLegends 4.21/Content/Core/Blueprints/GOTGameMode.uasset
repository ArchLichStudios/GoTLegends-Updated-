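; Game mode for a Game of Thrones hero-collection game that owns the player profile and syncs it with GameSparks.
; BeginPlay connects, shows splash, login and menu widgets, and spawns a data holder actor per character table row.
; After authentication it loads player, guild and hero data into its variables and those holders.
; Currency, XP, energy and power helpers change local values and mostly send deltas to the server; Tick drives an energy regen countdown.
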(event `PlayMusic`
  (`GameplayStatics.PlaySound2D` "/Game/Core/AudioTracks/1-TV_Themes_-_Game_Of_Thrones_Main_Title_Theme.1-TV_Themes_-_Game_Of_Thrones_Main_Title_Theme" 1.0 1.0 0.0 null null))

(event `self.ReceiveBeginPlay`
  (bind _gamesparks (`self.GameSparks`))
  ;[1 1 1] Loads The Beginning of Game Splash Screen
  (bind _returnvalue (`|CreateWidget` "/Game/Core/UI/SplashScreen.SplashScreen_C"))
  (`UserWidget.AddToViewport` _returnvalue 30)
  ;[1 1 1] Connect to Server
  (`GameSparksComponent.Disconnect` _gamesparks)
  (`GameSparksComponent.Connect` _gamesparks (`self.APIKey`) (`self.SecretKey`) true true)
  ;[1 1 1] Create Login Widget
  (bind _returnvalue_2 (`|CreateWidget` "/Game/Core/UI/Widgets_Login/GameSparksLogin.GameSparksLogin_C"))
  (`UserWidget.AddToViewport` _returnvalue_2 20)
  ;[1 1 1] Create Main Menu Widget & Set Ref
  (bind _returnvalue_3 (`|CreateWidget` "/Game/Core/UI/Widgets_MainMenu/Widget_MainMenu.Widget_MainMenu_C"))
  (`UserWidget.AddToViewport` _returnvalue_3 0)
  (set `self.MainMenuRef` _returnvalue_3)
  (`self.Spawn Data Holders`) ; Spawn Data Holder Actors
  (`KismetSystemLibrary.Delay` 3.0)
  (`self.PlayMusic`))

(event `self.GameSparks.OnGameSparksAvailableDelegate`
  (params (available :type Boolean))
  ;[1 1 1] Check Server Status
  (if available
    (`KismetSystemLibrary.PrintString` "Server Status: Available" true true (struct :`R` 0.006835 :`G` 0.53125 :`A` 1.0) 5.0)
    (else
      (`KismetSystemLibrary.PrintString` "Server Status: Unavailable" true true (struct :`R` 0.348958 :`G` 0.01452 :`B` 0.017991 :`A` 1.0) 5.0))))

(event `GetHeroes`
  (bind _returnvalue (`GameSparksComponent.IsAuthenticated` (`self.GameSparks`)))
  (if _returnvalue
    (bind _logeventresponse (`GSLogEventRequest.SendLogEventRequest` "GetUserHeros" null)
      (:`then`
        (`KismetSystemLibrary.PrintString` "Get Heroes No Response"))
      (:`OnResponse`
        (for _array_element (`GameSparksScriptData.GetGSDataArray` (`.ScriptData` (break `GSLogEventResponse` _logeventresponse)) "UserHeros")
          (bind _returnvalue_2 (`|GetDataTableRow` "/Game/Core/DataBPs/DataTable_CharacterTable.DataTable_CharacterTable" (`KismetStringLibrary.Conv_StringToName` (`GameSparksScriptData.GetString` _array_element "HeroID")))
            (:`then`
              (bind _outactors (`GameplayStatics.GetAllActorsOfClass` (`.DataHolderReference_21_81A2D21C4DFC6C0D74DE43A2260FCF64` (break `/Game/Core/DataBPs/Struct_CharInfo` _returnvalue_2))))
              (bind _output (`|GetArrayItem` _outactors))
              (set `/Game/Core/MasterClassBPs/CharDataHolder_MasterClass.Gamesparks Hero ID` (`GameSparksScriptData.GetString` _array_element "ID") _output)
              (set `/Game/Core/MasterClassBPs/CharDataHolder_MasterClass.Shards` (`KismetMathLibrary.Conv_IntToDouble` (`GameSparksScriptData.GetNumber` _array_element "Shards")) _output)
              (if (`GameSparksScriptData.GetBoolean` _array_element "Unlocked")
                (set `/Game/Core/MasterClassBPs/CharDataHolder_MasterClass.CharLocked?` "NewEnumerator1" _output)
                (set `/Game/Core/MasterClassBPs/CharDataHolder_MasterClass.Power` (`KismetMathLibrary.Conv_IntToDouble` (`GameSparksScriptData.GetNumber` _array_element "Power")) _output)
                (bind _star_output (`self.CalculateStarsForGS` (`GameSparksScriptData.GetNumber` _array_element "Stars")))
                (set `/Game/Core/MasterClassBPs/CharDataHolder_MasterClass.StarLevel` _star_output _output)))
            (:`RowNotFound`
              (`KismetSystemLibrary.PrintString` "RowNotFound"))))))))

(event `GetPlayerData`
  (bind _logeventresponse (`GSLogEventRequest.SendLogEventRequest` "GetPlayerInfo" (`GameSparksLogEventData.SetString` (`GameSparksLogEventData.CreateGameSparksLogEventAttributes`) "playerID" (`self.PlayerID`)))
    (:`OnResponse`
      (bind _returnvalue (`GameSparksScriptData.GetGSData` (`GameSparksScriptData.GetGSData` (`.ScriptData` (break `GSLogEventResponse` _logeventresponse)) "entry") "data"))
      (set `self.PlayerLevel` (`KismetMathLibrary.Conv_IntToDouble` (`GameSparksScriptData.GetNumber` _returnvalue "Level")))
      (set `self.TotalCollectionPower` (`KismetMathLibrary.Conv_IntToDouble` (`GameSparksScriptData.GetNumber` _returnvalue "TotalCollectionPower")))
      (set `self.PlayerMaxXP` (`KismetMathLibrary.Conv_IntToDouble` (`GameSparksScriptData.GetNumber` _returnvalue "MaxXP")))
      (set `self.MaxEnergy` (`KismetMathLibrary.Conv_IntToDouble` (`GameSparksScriptData.GetNumber` _returnvalue "MaxEnergy")))
      (set `self.HeroesUnlocked` (`KismetMathLibrary.Conv_IntToDouble` (`GameSparksScriptData.GetNumber` _returnvalue "HeroesCollected")))
      (set `self.PlayerXP` (`KismetMathLibrary.Conv_IntToDouble` (`GameSparksScriptData.GetNumber` _returnvalue "XP")))
      (set `self.Energy` (`KismetMathLibrary.Conv_IntToDouble` (`GameSparksScriptData.GetNumber` _returnvalue "Energy")))
      (set `self.Gold` (`KismetMathLibrary.Conv_IntToDouble` (`GameSparksScriptData.GetNumber` _returnvalue "Gold")))
      (set `self.Gems` (`KismetMathLibrary.Conv_IntToDouble` (`GameSparksScriptData.GetNumber` _returnvalue "Gems")))
      (`self.SetLeaderBoardScore`))))

(event `Check For Guild`
  ;[1 1 1] Checks to see if player is in a guild from GS server, if so, sets the "Guild Vars"
  ;;[1 1 1] Check if player is authenticated
  (bind _returnvalue (`GameSparksComponent.IsAuthenticated` (`self.GameSparks`)))
  (if _returnvalue
    (bind _getmyteamsresponse (`GSGetMyTeamsRequest.SendGetMyTeamsRequest` false null null)
      (:`OnResponse`
        (bind ((`HasTeams` _hasteams) (`Teams` _teams)) (break `GSGetMyTeamsResponse` _getmyteamsresponse))
        (if _hasteams
          (set `self.Has Guild?` true)
          (bind ((`HasMembers` _hasmembers) (`Members` _members) (`Owner` _owner) (`TeamId` _teamid) (`TeamName` _teamname)) (break `GSTeam` (`|GetArrayItem` _teams)))
          (set `self.GuildName` (`KismetTextLibrary.Conv_StringToText` _teamname))
          (set `self.GuildID` _teamid)
          (set `self.GuildOwnerID` (`.Id` (break `GSPlayer` _owner)))
          (else
            (set `self.Has Guild?` false)
            (set `self.GuildName` "")
            (set `self.GuildID` "")
            (set `self.GuildOwnerID` "")))))
    (else
      ;;[1 1 1] Keeps repeating check until player is authenticated
      (`KismetSystemLibrary.Delay` 0.2)
      (`self.Check For Guild`))))

(event `Server Synch - Total Collection Power`
  (params (`TCP To Add` :type Integer))
  (`KismetSystemLibrary.PrintString` (`KismetTextLibrary.Conv_TextToString` (`|FormatText` "Levels To Add: {a}" `TCP To Add`)))
  (`GSLogEventRequest.SendLogEventRequest` "updatePlayerData" (`GameSparksLogEventData.SetNumber` (`GameSparksLogEventData.SetNumber` (`GameSparksLogEventData.SetNumber` (`GameSparksLogEventData.SetNumber` (`GameSparksLogEventData.SetNumber` (`GameSparksLogEventData.SetNumber` (`GameSparksLogEventData.SetNumber` (`GameSparksLogEventData.SetNumber` (`GameSparksLogEventData.SetNumber` (`GameSparksLogEventData.SetNumber` (`GameSparksLogEventData.CreateGameSparksLogEventAttributes`) "Level" 0) "TotalCollectionPower" `TCP To Add`) "XP" 0) "MaxXP" 0) "StrongestTeamPower" 0) "HeroesCollected" 0) "Energy" 0) "MaxEnergy" 0) "Gems" 0) "Gold" 0)))

(event `self.GSMessageListeners.OnTeamChatMessage`
  (params (TeamChatMessage :type "GSTeamChatMessage Structure"))
  (bind ((`Message` _message) (`Who` _who)) (break `GSTeamChatMessage` TeamChatMessage))
  (bind _housemenuref (`self.HouseMenuRef`))
  ;[1 1 1] Gets a list of player's guild messages to populate Guild Chat Box
  (`/Game/Core/UI/Widgets_Social/Widget_HouseMenu.RefreshChat` _housemenuref (`KismetTextLibrary.Conv_StringToText` _who) (`KismetTextLibrary.Conv_StringToText` _message))
  (`ScrollBox.ScrollToEnd` (`/Game/Core/UI/Widgets_Social/Widget_HouseMenu.ChatBox` _housemenuref)))

(event `UserComeOnlineGuildMessage`
  (`GSSendTeamChatMessageRequest.SendSendTeamChatMessageRequest` (`KismetTextLibrary.Conv_TextToString` (`|FormatText` "{Username} has come online" (`self.Username`))) (`self.GuildOwnerID`) (`self.GuildID`) "GUILD" (`GameSparksScriptData.CreateGameSparksScriptData`)))

(event `Server Synch - Player Level`
  (params (`Levels To Add` :type Integer) (`MaxXP to Add` :type Integer) (`MaxEnergy to Add` :type Integer))
  (`KismetSystemLibrary.PrintString` (`KismetTextLibrary.Conv_TextToString` (`|FormatText` "Levels To Add: {a}" `Levels To Add`)))
  (`GSLogEventRequest.SendLogEventRequest` "updatePlayerData" (`GameSparksLogEventData.SetNumber` (`GameSparksLogEventData.SetNumber` (`GameSparksLogEventData.SetNumber` (`GameSparksLogEventData.SetNumber` (`GameSparksLogEventData.SetNumber` (`GameSparksLogEventData.SetNumber` (`GameSparksLogEventData.SetNumber` (`GameSparksLogEventData.SetNumber` (`GameSparksLogEventData.SetNumber` (`GameSparksLogEventData.SetNumber` (`GameSparksLogEventData.CreateGameSparksLogEventAttributes`) "Level" `Levels To Add`) "TotalCollectionPower" 0) "XP" 0) "MaxXP" `MaxXP to Add`) "StrongestTeamPower" 0) "HeroesCollected" 0) "Energy" 0) "MaxEnergy" `MaxEnergy to Add`) "Gems" 0) "Gold" 0)))

(event `UnlockHero`
  (params (ID :type Name))
  (bind (_logeventresponse _haserrors) (`GSLogEventRequest.SendLogEventRequest` "UnlockHero" (`GameSparksLogEventData.SetString` (`GameSparksLogEventData.CreateGameSparksLogEventAttributes`) "HeroID" (`KismetStringLibrary.Conv_NameToString` ID)))
    (:`OnResponse`
      (if (not _haserrors)
        (bind _returnvalue (`|GetDataTableRow` "/Game/Core/DataBPs/DataTable_CharacterTable.DataTable_CharacterTable" ID)
          (:`then`
            (bind (_errors _hasrequestid _requestid _hasscriptdata _scriptdata _jsonstring) (break `GSLogEventResponse` _logeventresponse))
            (`KismetSystemLibrary.PrintString` _jsonstring true true (struct :`G` 0.66 :`B` 1.0 :`A` 1.0) 20.0)
            (bind _outactors (`GameplayStatics.GetAllActorsOfClass` (`.DataHolderReference_21_81A2D21C4DFC6C0D74DE43A2260FCF64` (break `/Game/Core/DataBPs/Struct_CharInfo` _returnvalue))))
            (bind _returnvalue_2 (`GameSparksScriptData.GetGSData` _scriptdata "UserHero"))
            (bind _returnvalue_3 (`GameSparksScriptData.GetNumber` (`GameSparksScriptData.GetGSData` _returnvalue_2 "data") "Power"))
            (`KismetSystemLibrary.PrintString` (`KismetTextLibrary.Conv_TextToString` (`|FormatText` "Server Power: {a}" (`KismetTextLibrary.Conv_StringToText` (`KismetStringLibrary.Conv_IntToString` _returnvalue_3)))))
            (bind _output (`|GetArrayItem` _outactors))
            (set `/Game/Core/MasterClassBPs/CharDataHolder_MasterClass.CharLocked?` "NewEnumerator1" _output)
            (bind _output_get (set `/Game/Core/MasterClassBPs/CharDataHolder_MasterClass.Gamesparks Hero ID` (`GameSparksScriptData.GetString` _returnvalue_2 "id") _output))
            (bind _output_get_2 (set `/Game/Core/MasterClassBPs/CharDataHolder_MasterClass.Power` (`KismetMathLibrary.Conv_IntToDouble` _returnvalue_3) _output))
            (`self.Add To Total Collection Powr` _output_get_2)
            (`KismetSystemLibrary.PrintString` (`KismetTextLibrary.Conv_TextToString` (`|FormatText` "ID Set To:{a}" (`KismetTextLibrary.Conv_StringToText` _output_get))))
            (set `self.HeroesUnlocked` (+ (`self.HeroesUnlocked`) 1.0))))))))

(event `Server Synch - Add Energy`
  (params (Energy :type Integer))
  (`KismetSystemLibrary.PrintString` (`KismetTextLibrary.Conv_TextToString` (`|FormatText` "Levels To Add: {a}" _)))
  (`GSLogEventRequest.SendLogEventRequest` "updatePlayerData" (`GameSparksLogEventData.SetNumber` (`GameSparksLogEventData.SetNumber` (`GameSparksLogEventData.SetNumber` (`GameSparksLogEventData.SetNumber` (`GameSparksLogEventData.SetNumber` (`GameSparksLogEventData.SetNumber` (`GameSparksLogEventData.SetNumber` (`GameSparksLogEventData.SetNumber` (`GameSparksLogEventData.SetNumber` (`GameSparksLogEventData.SetNumber` (`GameSparksLogEventData.CreateGameSparksLogEventAttributes`) "Level" 0) "TotalCollectionPower" 0) "XP" 0) "MaxXP" 0) "StrongestTeamPower" 0) "HeroesCollected" 0) "Energy" Energy) "MaxEnergy" 0) "Gems" 0) "Gold" 0)))

(event `Server Synch Remove Energy`
  (params (Energy :type Integer))
  (bind _result (`/Engine/EditorBlueprintResources/StandardMacros.NegateInt` Energy)
    (:`  `
      (`GSLogEventRequest.SendLogEventRequest` "updatePlayerData" (`GameSparksLogEventData.SetNumber` (`GameSparksLogEventData.SetNumber` (`GameSparksLogEventData.SetNumber` (`GameSparksLogEventData.SetNumber` (`GameSparksLogEventData.SetNumber` (`GameSparksLogEventData.SetNumber` (`GameSparksLogEventData.SetNumber` (`GameSparksLogEventData.SetNumber` (`GameSparksLogEventData.SetNumber` (`GameSparksLogEventData.SetNumber` (`GameSparksLogEventData.CreateGameSparksLogEventAttributes`) "Level" 0) "TotalCollectionPower" 0) "XP" 0) "MaxXP" 0) "StrongestTeamPower" 0) "HeroesCollected" 0) "Energy" _result) "MaxEnergy" 0) "Gems" 0) "Gold" 0)))))

(event `self.ReceiveTick`
  (params (DeltaSeconds :type "Float (single-precision)"))
  (bind _minutes (`self.Minutes`))
  (`KismetSystemLibrary.Delay` 1.0)
  (if (and (== (`self.Seconds`) 0.0) (== (`self.Minutes`) 0.0))
    (`self.Add Energy` 1.0))
  (if (<= (`self.Seconds`) 0.0)
    (set `self.Seconds` 59.0)
    (if (>= _minutes 1.0)
      (set `self.Minutes` (- _minutes 1.0))
      (else
        (set `self.Minutes` 4.0)))
    (else
      (set `self.Seconds` (- (`self.Seconds`) 1.0)))))

(event `ServerSynch - Add Gems`
  (params (Gems :type Integer))
  (`GSLogEventRequest.SendLogEventRequest` "updatePlayerData" (`GameSparksLogEventData.SetNumber` (`GameSparksLogEventData.SetNumber` (`GameSparksLogEventData.SetNumber` (`GameSparksLogEventData.SetNumber` (`GameSparksLogEventData.SetNumber` (`GameSparksLogEventData.SetNumber` (`GameSparksLogEventData.SetNumber` (`GameSparksLogEventData.SetNumber` (`GameSparksLogEventData.SetNumber` (`GameSparksLogEventData.SetNumber` (`GameSparksLogEventData.CreateGameSparksLogEventAttributes`) "Level" 0) "TotalCollectionPower" 0) "XP" 0) "MaxXP" 0) "StrongestTeamPower" 0) "HeroesCollected" 0) "Energy" 0) "MaxEnergy" 0) "Gems" Gems) "Gold" 0)))

(event `Server Synch - Add Gold`
  (params (Gold :type Integer))
  (`GSLogEventRequest.SendLogEventRequest` "updatePlayerData" (`GameSparksLogEventData.SetNumber` (`GameSparksLogEventData.SetNumber` (`GameSparksLogEventData.SetNumber` (`GameSparksLogEventData.SetNumber` (`GameSparksLogEventData.SetNumber` (`GameSparksLogEventData.SetNumber` (`GameSparksLogEventData.SetNumber` (`GameSparksLogEventData.SetNumber` (`GameSparksLogEventData.SetNumber` (`GameSparksLogEventData.SetNumber` (`GameSparksLogEventData.CreateGameSparksLogEventAttributes`) "Level" 0) "TotalCollectionPower" 0) "XP" 0) "MaxXP" 0) "StrongestTeamPower" 0) "HeroesCollected" 0) "Energy" 0) "MaxEnergy" 0) "Gems" 0) "Gold" Gold)))

(event `SetLeaderBoardScore`
  (`GSLogEventRequest.SendLogEventRequest` "TCPLeaderBoardScorer" (`GameSparksLogEventData.SetNumber` (`GameSparksLogEventData.CreateGameSparksLogEventAttributes`) "Scorer" (`KismetMathLibrary.FTrunc` (`self.TotalCollectionPower`)))))

(event `ServerSynch - Add XP`
  (params (XP :type Integer))
  (`GSLogEventRequest.SendLogEventRequest` "updatePlayerData" (`GameSparksLogEventData.SetNumber` (`GameSparksLogEventData.SetNumber` (`GameSparksLogEventData.SetNumber` (`GameSparksLogEventData.SetNumber` (`GameSparksLogEventData.SetNumber` (`GameSparksLogEventData.SetNumber` (`GameSparksLogEventData.SetNumber` (`GameSparksLogEventData.SetNumber` (`GameSparksLogEventData.SetNumber` (`GameSparksLogEventData.SetNumber` (`GameSparksLogEventData.CreateGameSparksLogEventAttributes`) "Level" 0) "TotalCollectionPower" 0) "XP" XP) "MaxXP" 0) "StrongestTeamPower" 0) "HeroesCollected" 0) "Energy" 0) "MaxEnergy" 0) "Gems" 0) "Gold" 0)))

(event `Server Synch - Remove XP`
  (params (XP :type Integer))
  (bind _result (`/Engine/EditorBlueprintResources/StandardMacros.NegateInt` XP)
    (:`  `
      (`GSLogEventRequest.SendLogEventRequest` "updatePlayerData" (`GameSparksLogEventData.SetNumber` (`GameSparksLogEventData.SetNumber` (`GameSparksLogEventData.SetNumber` (`GameSparksLogEventData.SetNumber` (`GameSparksLogEventData.SetNumber` (`GameSparksLogEventData.SetNumber` (`GameSparksLogEventData.SetNumber` (`GameSparksLogEventData.SetNumber` (`GameSparksLogEventData.SetNumber` (`GameSparksLogEventData.SetNumber` (`GameSparksLogEventData.CreateGameSparksLogEventAttributes`) "Level" 0) "TotalCollectionPower" 0) "XP" _result) "MaxXP" 0) "StrongestTeamPower" 0) "HeroesCollected" 0) "Energy" 0) "MaxEnergy" 0) "Gems" 0) "Gold" 0)))))

(fn `Add Energy`
  (params (Amount :type "Float (double-precision)"))
  (set `self.Energy` (+ (`self.Energy`) Amount))
  (`self.Server Synch - Add Energy` (`KismetMathLibrary.FTrunc` Amount)))

(fn `Add Gems`
  (params (Amount :type "Float (double-precision)"))
  (set `self.Gems` (+ (`self.Gems`) Amount))
  (`self.ServerSynch - Add Gems` (`KismetMathLibrary.FTrunc` Amount)))

(fn `Add Gold`
  (params (Amount :type "Float (double-precision)"))
  (set `self.Gold` (+ (`self.Gold`) Amount))
  (`self.Server Synch - Add Gold` (`KismetMathLibrary.FTrunc` Amount)))

(fn `Add Shards`
  (params (`Char ID:` :type Name) (Amount :type "Float (double-precision)"))
  (locals (`Local Shards` :type "Float (double-precision)"))
  ;[1 1 1] Gets Character Reference for Selected Character
  (bind _returnvalue (`|GetDataTableRow` "/Game/Core/DataBPs/DataTable_CharacterTable.DataTable_CharacterTable" `Char ID:`)
    (:`then`
      (bind _outactors (`GameplayStatics.GetAllActorsOfClass` (`.DataHolderReference_21_81A2D21C4DFC6C0D74DE43A2260FCF64` (break `/Game/Core/DataBPs/Struct_CharInfo` _returnvalue))))
      (`/Game/Core/MasterClassBPs/CharDataHolder_MasterClass.Add Shards` (`|GetArrayItem` _outactors) Amount))))

(fn `Add Stars`
  (params (`Char ID:` :type Name) (Amount :type "/Game/Core/DataBPs/Enum_CharStarLevel Enum" :default "NewEnumerator0"))
  (locals (`Local Shards` :type "Float (double-precision)"))
  ;[1 1 1] Gets Character Reference for Selected Character
  (bind _returnvalue (`|GetDataTableRow` "/Game/Core/DataBPs/DataTable_CharacterTable.DataTable_CharacterTable" `Char ID:`)
    (:`then`
      (bind _outactors (`GameplayStatics.GetAllActorsOfClass` (`.DataHolderReference_21_81A2D21C4DFC6C0D74DE43A2260FCF64` (break `/Game/Core/DataBPs/Struct_CharInfo` _returnvalue))))
      (`/Game/Core/MasterClassBPs/CharDataHolder_MasterClass.Add Stars` (`|GetArrayItem` _outactors) Amount))))

(fn `Add To Total Collection Powr`
  (params (Amount :type "Float (double-precision)"))
  (set `self.TotalCollectionPower` (+ (`self.TotalCollectionPower`) Amount))
  (`KismetSystemLibrary.PrintString` (`KismetTextLibrary.Conv_TextToString` (`|FormatText` "TCP Added:{a}" Amount)))
  (`self.Server Synch - Total Collection Power` (`KismetMathLibrary.FTrunc` Amount))
  (`self.SetLeaderBoardScore`))

(fn `Add XP`
  (params (Amount :type "Float (double-precision)"))
  (bind _output_get (set `self.PlayerXP` (+ (`self.PlayerXP`) Amount)))
  (if (>= _output_get (`self.PlayerMaxXP`))
    (`self.Profile Level Up`)
    (else
      (`self.ServerSynch - Add XP` (`KismetMathLibrary.FTrunc` Amount)))))

(fn `AddPower`
  (params (`Char ID:` :type Name) (Amount :type "Float (double-precision)"))
  (locals (`Local Shards` :type "Float (double-precision)"))
  ;[1 1 1] Gets Character Reference for Selected Character
  (bind _returnvalue (`|GetDataTableRow` "/Game/Core/DataBPs/DataTable_CharacterTable.DataTable_CharacterTable" `Char ID:`)
    (:`then`
      (bind _outactors (`GameplayStatics.GetAllActorsOfClass` (`.DataHolderReference_21_81A2D21C4DFC6C0D74DE43A2260FCF64` (break `/Game/Core/DataBPs/Struct_CharInfo` _returnvalue))))
      (`/Game/Core/MasterClassBPs/CharDataHolder_MasterClass.Add Power` (`|GetArrayItem` _outactors) Amount))))

(fn `AfterAuthenticatedEvents`
  (`self.GetPlayerData`)
  (`self.Check For Guild`)
  (`self.GetHeroes`)
  (`self.UserComeOnlineGuildMessage`))

(fn `CalculateStarsForGS`
  (params (`Stars Input` :type Integer))
  (returns (`Star Output` :type "/Game/Core/DataBPs/Enum_CharStarLevel Enum"))
  (if (== `Stars Input` 1)
    (return "NewEnumerator1")
    (elif (== `Stars Input` 2)
      (return "NewEnumerator2")
      (elif (== `Stars Input` 3)
        (return "NewEnumerator3")
        (elif (== `Stars Input` 4)
          (return "NewEnumerator4")
          (elif (== `Stars Input` 5)
            (return "NewEnumerator5")
            (elif (== `Stars Input` 6)
              (return "NewEnumerator6")
              (elif (== `Stars Input` 7)
                (return "NewEnumerator7")
                (else
                  (`KismetSystemLibrary.PrintString` "Failure To Convert"))))))))))

(fn `Profile Level Up`
  (bind _playermaxxp (`self.PlayerMaxXP`))
  (bind _output_get (set `self.MaxEnergy` (+ (`self.MaxEnergy`) 5.0)))
  (`self.Add Energy` _output_get)
  (`self.Remove XP` _playermaxxp)
  (set `self.PlayerMaxXP` (+ _playermaxxp 50.0))
  (bind _output_get_2 (set `self.PlayerLevel` (+ (`self.PlayerLevel`) 1.0)))
  (`self.Add Gems` 20.0)
  (`self.Add Gold` 1000.0)
  (bind _returnvalue (`|CreateWidget` "/Game/Core/UI/Widget_PlayerLevelUp.Widget_PlayerLevelUp_C" null _output_get_2 (`self.MaxEnergy`)))
  (`UserWidget.AddToViewport` _returnvalue 20)
  (`self.Server Synch - Player Level` 1 50 5))

(fn `Remove Energy`
  (params (Amount :type "Float (double-precision)"))
  (bind _energy (`self.Energy`))
  (set `self.Energy` (- _energy Amount))
  (if (< _energy 0.0)
    (set `self.Energy` 0.0)
    (else
      (`self.Server Synch Remove Energy` (`KismetMathLibrary.FTrunc` Amount)))))

(fn `Remove Gold`
  (params (Amount :type "Float (double-precision)"))
  (bind _output_get (set `self.Gold` (- (`self.Gold`) Amount)))
  (if (<= _output_get 0.0)
    (set `self.Gold` 0.0)))

(fn `Remove Shards`
  (params (`Char ID:` :type Name) (Amount :type "Float (double-precision)"))
  (locals (`Local Shards` :type "Float (double-precision)"))
  ;[1 1 1] Gets Character Reference for Selected Character
  (bind _returnvalue (`|GetDataTableRow` "/Game/Core/DataBPs/DataTable_CharacterTable.DataTable_CharacterTable" `Char ID:`)
    (:`then`
      (bind _outactors (`GameplayStatics.GetAllActorsOfClass` (`.DataHolderReference_21_81A2D21C4DFC6C0D74DE43A2260FCF64` (break `/Game/Core/DataBPs/Struct_CharInfo` _returnvalue))))
      (`/Game/Core/MasterClassBPs/CharDataHolder_MasterClass.Remove Shards` (`|GetArrayItem` _outactors) Amount))))

(fn `Remove XP`
  (params (Amount :type "Float (double-precision)"))
  (bind _playerxp (`self.PlayerXP`))
  (set `self.PlayerXP` (- _playerxp Amount))
  (if (< _playerxp 0.0)
    (set `self.PlayerXP` 0.0)
    (else
      (`self.Server Synch - Remove XP` (`KismetMathLibrary.FTrunc` Amount)))))

(fn `RemoveGems`
  (params (Amount :type "Float (double-precision)"))
  (set `self.Gems` (- (`self.Gems`) Amount)))

(fn `Return To Main Menu`
  (`WidgetLayoutLibrary.RemoveAllWidgets`)
  (bind _returnvalue (`|CreateWidget` "/Game/Core/UI/Widgets_MainMenu/Widget_MainMenu.Widget_MainMenu_C"))
  (bind _output_get (set `self.MainMenuRef` _returnvalue))
  (`UserWidget.AddToViewport` _output_get 0))

(fn `Spawn Data Holders`
  (locals (SpawnLocation :type "Vector Structure" :default (11200.0 49080.0 34650.0)))
  ;[1 1 1] Gets Data for Each Character in the Character Database - Spawns "Data Holder" object to track stats for each character
  (bind _outrownames (`DataTableFunctionLibrary.GetDataTableRowNames` "/Game/Core/DataBPs/DataTable_CharacterTable.DataTable_CharacterTable"))
  (for _array_element _outrownames
    (bind _returnvalue (`|GetDataTableRow` "/Game/Core/DataBPs/DataTable_CharacterTable.DataTable_CharacterTable" _array_element)
      (:`then`
        (bind (_id _name _icon _loadingscreenart _heroid _characterreleased_ _characterbpreference _dataholderreference _charscreenmodelreference _shipreference _starlevelunlockedat _charactertype _leadercharacter_ _captaincharacter_ _herovillain _greathouse _house _organization _region) (break `/Game/Core/DataBPs/Struct_CharInfo` _returnvalue))
        (`|SpawnActorFromClass` _dataholderreference (`KismetMathLibrary.MakeTransform` (`local.SpawnLocation`)) "AlwaysSpawn" "OverrideRootScale" null (make `/Game/Core/DataBPs/Struct_CharInfo` _id _name _icon _loadingscreenart _heroid _characterreleased_ _characterbpreference _dataholderreference _charscreenmodelreference _shipreference _starlevelunlockedat _charactertype _leadercharacter_ _captaincharacter_ _herovillain _greathouse _house _organization _region) "" null)))))

(fn `UserConstructionScript`)